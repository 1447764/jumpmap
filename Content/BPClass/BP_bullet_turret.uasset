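; Turret actor that detects player-tagged actors with a sphere collider and fires BP_bullet at them.
; Entering the sphere stores the target and starts looping rotate and shoot timers; leaving clears both.
; Rotate computes a look-at rotation from turret to target but applies it to the target, not the turret.
; Shoot line-traces to the target and spawns a bullet at the turret's transform on a player hit.
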(event `self.SphereCollider.OnComponentBeginOverlap`
  (params (OverlappedComponent :type "PrimitiveComponent Object Reference") (OtherActor :type "Actor Object Reference") (OtherComp :type "PrimitiveComponent Object Reference") (OtherBodyIndex :type Integer) (bFromSweep :type Boolean) (SweepResult :type "HitResult Structure (by ref)"))
  (`/Engine/EditorBlueprintResources/StandardMacros.IsValid` OtherActor
    (:`Is Valid`
      (if (`self.ActorHasTag` OtherActor "player")
        (set `self.Target` OtherActor)
        (`self.Track Target`)))))

(event `self.SphereCollider.OnComponentEndOverlap`
  (params (OverlappedComponent :type "PrimitiveComponent Object Reference") (OtherActor :type "Actor Object Reference") (OtherComp :type "PrimitiveComponent Object Reference") (OtherBodyIndex :type Integer))
  (`/Engine/EditorBlueprintResources/StandardMacros.IsValid` OtherActor
    (:`Is Valid`
      (if (`self.ActorHasTag` OtherActor "player")
        (`self.Target`
          (:`then`
            (`KismetSystemLibrary.K2_ClearAndInvalidateTimerHandle` (`self.Timer_Rotate`))
            (`KismetSystemLibrary.K2_ClearAndInvalidateTimerHandle` (`self.Timer_Shoot`)))
          (:`else`))))))

(event `Track Target`
  (bind _returnvalue (`KismetSystemLibrary.K2_SetTimerDelegate` (delegate `Rotate`) 0.05 true true))
  (set `self.Timer_Rotate` _returnvalue)
  (bind _returnvalue_2 (`KismetSystemLibrary.K2_SetTimerDelegate` (delegate `Shoot`) 1.0 true true))
  (set `self.Timer_Shoot` _returnvalue_2))

(event `Rotate`
  (bind _target (`self.Target`))
  (`/Engine/EditorBlueprintResources/StandardMacros.IsValid` _target
    (:`Is Valid`
      (`self.K2_SetActorRelativeRotation` (`self.Target`) (`KismetMathLibrary.RInterpTo` (`SceneComponent.RelativeRotation` (`self.DefaultSceneRoot`)) (`KismetMathLibrary.FindLookAtRotation` (`self.K2_GetActorLocation`) (`self.K2_GetActorLocation` _target)) (`GameplayStatics.GetWorldDeltaSeconds`)) false false))))

(event `Shoot`
  (bind (_outhit _returnvalue) (`KismetSystemLibrary.LineTraceSingle` (+ (`self.K2_GetActorLocation`) (0.0 0.0 0.0)) (`self.K2_GetActorLocation` (`self.Target`)) "TraceTypeQuery2" true))
  (if _returnvalue
    (if (`self.ActorHasTag` (`.HitActor` (`GameplayStatics.BreakHitResult` _outhit)) "player")
      (`|SpawnActorFromClass` "/Game/BPClass/BP_bullet.BP_bullet_C" (`self.GetTransform`) "Undefined" "MultiplyWithRoot" null null))))

(fn `UserConstructionScript`)